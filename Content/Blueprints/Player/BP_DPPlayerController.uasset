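; Player controller that shows a custom mouse cursor widget for the local player.
; BeginPlay creates the Mousecursor widget and adds it to the viewport.
; Tick moves the widget to the current mouse position each frame, removing DPI scale.
; Unconnected nodes that project the under-cursor trace hit to screen space are left in the graph and play no part.
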(event EventBeginPlay
  (if (Pawn|IsLocalPlayerController)
    (bind _returnvalue (UserInterface|CreateWidget "/Game/Blueprints/Widget/mousecursor.mousecursor_C" self))
    (bind _output_get (Variables|Default|SetCursorwidget _returnvalue))
    (UserInterface|Viewport|AddtoViewport _output_get 0)))

(event EventTick
  (params (DeltaSeconds :type Float%20%28single-precision%29))
  (bind (_locationx _locationy) (Game|Player|GetMousePosition))
  (if (Pawn|IsLocalPlayerController)
    (bind _cursorwidget (Variables|Default|GetCursorwidget)
      (:then
        (Class|UserWidget|SetPositioninViewport _cursorwidget (Math|Vector2D|MakeVector2D _locationx _locationy) true))
      (:else))))

(fn ConstructionScript)